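; BP_FlamePillar is a flame pillar actor whose fire light flickers continuously.
; On BeginPlay it randomly picks one of two intensity timelines, and each one picks again when it finishes, forming an endless, varied loop.
; While a timeline plays, its curve value is multiplied by BaseIntensity and applied to the FireLight component's intensity.
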(event Custom|IntensityWay1
  (bind _flameintensity (Timeline|FlameIntensity1 PlayFromStart)
    (:Update
      (CallFunction|UpdateIntensity _flameintensity))
    (:Finished
      (CallFunction|ChoseIntensityWay))))

(event Custom|IntensityWay2
  (bind _flameintensity (Timeline|FlameIntensity2 PlayFromStart)
    (:Update
      (CallFunction|UpdateIntensity _flameintensity))
    (:Finished
      (CallFunction|ChoseIntensityWay))))

(event Custom|ChoseIntensityWay
  (switch int (Math|Random|RandomIntegerinRange 0 1)
    (:0
      (CallFunction|IntensityWay1))
    (:1
      (CallFunction|IntensityWay2))))

(event EventBeginPlay
  (CallFunction|ChoseIntensityWay))

(fn ConstructionScript)

(fn UpdateIntensity
  (params (Intensity :type Float%20%28double-precision%29))
  (Rendering|Components|Light|SetIntensity (Variables|Default|GetFireLight) (* Intensity (Variables|Default|GetBaseIntensity))))