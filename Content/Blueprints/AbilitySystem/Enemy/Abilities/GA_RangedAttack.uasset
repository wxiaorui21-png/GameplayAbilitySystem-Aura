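; Enemy gameplay ability for a ranged attack that launches a projectile at the avatar's combat target.
; On activation it turns the avatar toward the target and plays a random tagged montage from the avatar's attack montages.
; The montage's gameplay event spawns the projectile at that montage's socket tag with an optional pitch override.
; The ability ends shortly after the shot, or when the montage completes, is interrupted or is cancelled.
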(event Ability|EventActivateAbility
  (bind _returnvalue (Ability|GetAvatarActorfromActorInfo))
  (bind _returnvalue_2 (Class|EnemyInterface|GetCombatTarget(Message) _returnvalue))
  (Class|CombatInterface|UpdateFacingTarget(Message) _returnvalue (Transformation|GetActorLocation _returnvalue_2))
  (bind _returnvalue_3 (Class|CombatInterface|GetAttackMontages(Message) (Ability|GetAvatarActorfromActorInfo)))
  (Variables|Default|SetAttackMontage (Class|AuraDamageGameplayAbility|GetRandomTaggedMontagefromArray _returnvalue_3))
  (|PlayMontageandWaitProxy "None" (.Montage (Utilities|Struct|BreakTaggedMontage (Variables|Default|GetAttackMontage))) 1.0 "None" false 1.0 0.0 false
    (:then
      (Ability|Tasks|WaitGameplayEvent (.MontageTag (Utilities|Struct|BreakTaggedMontage (Variables|Default|GetAttackMontage))) 0 true
        (:EventReceived
          (Class|AuraProjectileSpell|SpawnProjectile (Transformation|GetActorLocation _returnvalue_2) (.SocketTag (Utilities|Struct|BreakTaggedMontage (Variables|Default|GetAttackMontage))) (Variables|Default|GetIsOverridePitch) 25.0)
          (Utilities|FlowControl|Delay 0.5)
          (Ability|EndAbility))))
    (:OnCompleted
      (Ability|EndAbility :!label _label))
    (:OnInterrupted
      (goto _label))
    (:OnCancelled
      (goto _label))))

(event Ability|EventOnEndAbility
  (params (bWasCancelled :type Boolean)))