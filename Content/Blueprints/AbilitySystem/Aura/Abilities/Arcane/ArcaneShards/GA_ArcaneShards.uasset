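; Arcane Shards ability that shows a magic circle, then on press erupts a series of shards around the cursor location.
; A temporary points collection supplies randomly rotated ground points, their count set by ability level up to a cap.
; A montage event hides the circle, commits cost and starts a looping timer spawning one shard per point.
; Each shard damages and knocks back nearby characters and fires a GameplayCue; cooldown commits after the last.
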(event Custom|SpawnShards
  (if (< (Variables|Default|GetCount) (Variables|Default|GetSpawnCount))
    (CallFunction|SpawnArcaneShardsLocation)
    (CallFunction|SpawnIgnoreActors)
    (for _array_element (Variables|Default|GetIgnoreActors)
      (Class|AuraAbilitySystemLibrary|ApplyDamageEffect (Class|AuraDamageGameplayAbility|MakeDamageEffectParamsfromDefaultClass _array_element (Variables|Default|GetPointsLocation) true (- (Transformation|GetActorLocation _array_element) (Variables|Default|GetPointsLocation)) true (- (Transformation|GetActorLocation _array_element) (Variables|Default|GetPointsLocation)) true 35.0)))
    (Math|Integer|IncrementInt (Variables|Default|GetCount)
      (:%20%20
        (Class|GameplayAbility|ExecuteGameplayCuewithParams "(TagName=\"GameplayCue.ArcaneShards\")" (Ability|GameplayCue|MakeGameplayCueParameters :Location (Variables|Default|GetPointsLocation)))))
    (else
      (Utilities|Time|ClearandInvalidateTimerbyHandle (Variables|Default|GetTimeHandle))
      (Actor|DestroyActor (Variables|Default|GetPointsCollection))
      (Ability|CommitAbilityCooldown false)
      (Ability|EndAbility))))

(event Ability|EventActivateAbility
  (Class|GameplayAbility|CheckAbilityCost)
  (Utilities|FlowControl|Sequence
    (:then_0
      ;[0.02667 0.03094 0.15 0.5] 显示法阵
      (Class|PlayerInterface|ShowMagicCircle(Message) (Ability|GetAvatarActorfromActorInfo) 0))
    (:then_1
      (Ability|Tasks|WaitInputPress false
        (:OnPress
          ;[0.03502 0.15 0.04408 0.5] 获得鼠标位置
          (bind _datahandle (|CreatTargetDataUnderMouse)
            (:ValidData
              (bind _output_get (Variables|Default|SetMouseLocation (.Location (Collision|BreakHitResult (Ability|TargetData|GetHitResultfromTargetData _datahandle)))))
              (Class|CombatInterface|UpdateFacingTarget(Message) (Ability|GetAvatarActorfromActorInfo) _output_get)
              ;[0.15 0.04633 0.03148 0.5] 获得法术碎片生成点
              (bind _returnvalue (Game|SpawnActorfromClass "/Game/Blueprints/AbilitySystem/Aura/Abilities/Arcane/ArcaneShards/BP_PointsCollection.BP_PointsCollection_C" (Math|Transform|MakeTransform (Variables|Default|GetMouseLocation) "0, 0, 0" "1.000000,1.000000,1.000000") "AlwaysSpawn" "MultiplyWithRoot" 0 0))
              (bind _output_get_2 (Variables|Default|SetPointsCollection _returnvalue))
              (Variables|Default|SetSpawnCount (Math|Integer|Min(Integer) (Ability|GetAbilityLevel) (Variables|Default|GetNewCount)))
              (bind _returnvalue_2 (Class|PointCollection|GetGroundPoints _output_get_2 (Variables|Default|GetMouseLocation) (Variables|Default|GetSpawnCount) (Math|Random|RandomFloatinRange 0.0 3.6e+02)))
              (Variables|Default|SetPointsArray _returnvalue_2)
              (|PlayMontageandWaitProxy "None" "/Game/Assets/Characters/Aura/Animations/Abilities/AM_ArcaneShardss.AM_ArcaneShardss" 1.0 "None" true 1.0 0.0 false
                (:then
                  (Ability|Tasks|WaitGameplayEvent "(TagName=\"Event.Montage.ArcaneShards\")" 0 true
                    (:EventReceived
                      ;[0.03238 0.15 0.02455 0.5] 设置计时器以及生成第一个碎片
                      (bind _returnvalue_3 (Utilities|Time|SetTimerbyEvent (delegate Custom|SpawnShards) (Variables|Default|GetSpawnShardsTime) true))
                      (Variables|Default|SetTimeHandle _returnvalue_3)
                      (Class|PlayerInterface|HideMagicCircle(Message) (Ability|GetAvatarActorfromActorInfo))
                      (CallFunction|SpawnShards)
                      (Ability|CommitAbilityCost false))))))))))))

(fn SpawnArcaneShardsLocation
  (Variables|Default|SetPointsLocation (Transformation|GetWorldLocation (Utilities|Array|Get(acopy) (Variables|Default|GetPointsArray) (Variables|Default|GetCount)))))

(fn SpawnIgnoreActors
  (bind _returnvalue (Ability|GetAvatarActorfromActorInfo))
  (bind _outoverlappingactors (Class|AuraAbilitySystemLibrary|GetLiveCharacterwithinRadius _returnvalue (Utilities|Array|MakeArray _returnvalue) (Variables|Default|GetRadialDamageOuterRadius) (Variables|Default|GetPointsLocation)))
  (Variables|Default|SetIgnoreActors _outoverlappingactors))