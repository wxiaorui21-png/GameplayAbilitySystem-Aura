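; BP_FireBolt is the Fire Bolt ability's projectile actor, which explodes and removes itself once it stops moving.
; Each Tick it compares its current location with the previous frame's and treats movement at or below MinDistance as an impact.
; It then plays a 2D impact sound, spawns a Niagara fire explosion at that spot and destroys itself.
; This graph uses no overlap or hit events and applies no damage.
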(event EventBeginPlay)

(event Collision|EventActorBeginOverlap
  (params (OtherActor :type Actor%20Object%20Reference)))

(event EventTick
  (params (DeltaSeconds :type Float%20%28single-precision%29))
  (Variables|Default|SetActorLastLocation (Variables|Default|GetActorThisLocation))
  (Variables|Default|SetActorThisLocation (Transformation|GetActorLocation))
  (if (<= (Math|Vector|VectorLength (- (Variables|Default|GetActorThisLocation) (Variables|Default|GetActorLastLocation))) (Variables|Default|GetMinDistance))
    (Audio|PlaySound2D "/Game/Assets/Sounds/Abilities/FireBolt/sfx_FireBolt_Impact.sfx_FireBolt_Impact" 1.0 1.0 0.0 0 0)
    (Niagara|SpawnSystematLocation "/Game/Assets/Effects/Projectiles/FireExplosion/NS_FireExplosion1.NS_FireExplosion1" (Variables|Default|GetActorThisLocation))
    (Actor|DestroyActor)))

(fn ConstructionScript)