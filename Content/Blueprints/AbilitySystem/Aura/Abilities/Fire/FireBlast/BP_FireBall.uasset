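; BP_FireBall is a Fire Blast ability projectile that flies outward, returns to a target actor and explodes near it.
; On authority, one timeline lerps it to a forward apex, then another lerps it toward the moving ReturnToActor.
; Within explode distance it calls OnHit, applies radial damage effects to nearby living characters except its owner, with upward-pitched knockback and death impulse, then destroys itself.
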(event EventBeginPlay)

(event Collision|EventActorBeginOverlap
  (params (OtherActor :type Actor%20Object%20Reference)))

(event EventTick
  (params (DeltaSeconds :type Float%20%28single-precision%29)))

(event EventStartOutgoingTimeline
  (bind _returnvalue (Components|GetOwner))
  (bind _returnvalue_2 (CallFunction|OverridePitchDirection))
  (bind _array (Utilities|Array|MakeArray _returnvalue))
  (Networking|SwitchHasAuthority
    (:Authority
      ;[0.15 0.09127 0 0.5] 得到初始位置以及终点位置
      (Variables|Default|SetInitialLocation (Transformation|GetActorLocation))
      (Variables|Default|SetApexLocation (+ (* (Transformation|GetActorForwardVector) (Variables|Default|GetOutgoingDistance)) (Variables|Default|GetInitialLocation)))
      (bind _outgoingtrack (Timeline|OutgoingTimeline Play)
        (:Update
          (Transformation|SetActorLocation (Math|Vector|Lerp(Vector) (Variables|Default|GetInitialLocation) (Variables|Default|GetApexLocation) _outgoingtrack) false false))
        (:Finished
          (bind _returningtrack (Timeline|ReturningTimeline Play)
            (:Update
              (Transformation|SetActorLocation (Math|Vector|Lerp(Vector) (Transformation|GetActorLocation) (Transformation|GetActorLocation (Variables|Default|GetReturnToActor)) _returningtrack) false false)
              (if (CallFunction|IsShouldExplore)
                (Class|AuraProjectile|OnHit)
                (Class|AuraAbilitySystemLibrary|SetIsRadialDamageParams (Variables|Default|GetExplosionEffectParams) true 5e+01 1.5e+02 (Transformation|GetActorLocation))
                (Utilities|Array|Add _array self)
                (bind _outoverlappingactors (Class|AuraAbilitySystemLibrary|GetLiveCharacterwithinRadius self _array 1.5e+02 (Transformation|GetActorLocation)))
                (bind _output_get (Variables|Default|SetTargetActors _outoverlappingactors))
                (for _array_element _output_get
                  (Class|AuraAbilitySystemLibrary|SetAbilitySystemComponent (Variables|Default|GetExplosionEffectParams) (Ability|GetAbilitySystemComponent _array_element))
                  (Variables|Default|SetDirection (- (Transformation|GetActorLocation _array_element) (Transformation|GetActorLocation)))
                  (Class|AuraAbilitySystemLibrary|SetDeathImpulseDirection (Variables|Default|GetExplosionEffectParams) _returnvalue_2 (Variables|Default|GetDeathMagnitude))
                  (Class|AuraAbilitySystemLibrary|SetKnockBackDirection (Variables|Default|GetExplosionEffectParams) _returnvalue_2 (Variables|Default|GetKnockMagnitude))
                  (Class|AuraAbilitySystemLibrary|ApplyDamageEffect (Variables|Default|GetExplosionEffectParams)))
                (Actor|DestroyActor)))))))))

(fn ConstructionScript)

(fn IsShouldExplore
  (return (<= (Math|Vector|VectorLength (- (Transformation|GetActorLocation) (Transformation|GetActorLocation (Variables|Default|GetReturnToActor)))) (Variables|Default|GetExploreDistance))))

(fn OverridePitchDirection
  (bind _direction (Variables|Default|GetDirection))
  (bind _returnvalue (Math|Rotator|MakeRotfromX _direction))
  (return (Math|Vector|GetForwardVector (Math|Rotator|MakeRotator (.roll _returnvalue) 45.0 (.yaw _returnvalue)))))