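; GA_ListenForEvent is a passive startup gameplay ability that turns attribute gameplay events into changes on its owner.
; On activation it waits for events under the Attributes tag, child tags included, and builds a spec from a configured effect class for each event received.
; The event magnitude goes to its matching SetByCaller tag, with other listed tags zeroed to avoid errors, and the spec is applied to self.
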(event Ability|EventActivateAbility
  (bind _returnvalue (Ability|GetAbilitySystemComponentfromActorInfo))
  (Development|PrintString "ListenForEvent")
  (bind _payload (Ability|Tasks|WaitGameplayEvent "(TagName=\"Attributes\")" 0 false false)
    (:EventReceived
      (Variables|Default|SetEvent%20Tag (.EventTag (Utilities|Struct|BreakGameplayEventData _payload)))
      (Variables|Default|SetEvent%20Magnitude (.EventMagnitude (Utilities|Struct|BreakGameplayEventData _payload)))
      (Variables|Default|SetEffectSpec (GameplayEffects|MakeOutgoingSpec _returnvalue (Variables|Default|GetEvectBaseEffectClass) 0.0 (GameplayEffects|MakeEffectContext _returnvalue)))
      ;[0.15 0.15 0.15 0.5] 将其他不匹配的标签设置为0，目的是防止报错
      (for _array_element (Variables|Default|GetEventTags)
        (if (GameplayTags|MatchesTag _array_element (Variables|Default|GetEvent%20Tag) true)
          (Ability|GameplayEffect|AssignTagSetbyCallerMagnitude (Variables|Default|GetEffectSpec) (Variables|Default|GetEvent%20Tag) (Variables|Default|GetEvent%20Magnitude))
          (else
            (Ability|GameplayEffect|AssignTagSetbyCallerMagnitude (Variables|Default|GetEffectSpec) _array_element 0.0))))
      (GameplayEffects|ApplyGameplayEffectSpecToSelf (Ability|GetAbilitySystemComponentfromActorInfo) (Variables|Default|GetEffectSpec)))))

(event Ability|EventOnEndAbility
  (params (bWasCancelled :type Boolean)))