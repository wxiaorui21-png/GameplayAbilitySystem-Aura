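; BP_Aura_MainMenu is the main menu scene actor that shows the menu UI and animates magical decoration.
; On BeginPlay it plays menu music, adds WBP_MainMenu to the viewport and switches to UI-only input with the cursor shown.
; On Tick it bobs a Niagara component vertically on a sine wave from a wrapped time counter and steadily rolls a magic decal.
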(event EventBeginPlay
  (bind _returnvalue (Game|GetPlayerController 0))
  (Variables|Default|SetNiagaraInitLocation (Transformation|GetWorldLocation (Variables|Default|GetNiagara)))
  (Audio|PlaySound2D "/Game/Assets/Sounds/Music/Music_MainMenu.Music_MainMenu" 1.0 1.0 0.0 0 0)
  (bind _returnvalue_2 (UserInterface|CreateWidget "/Game/Blueprints/UI/MainMenu/WBP_MainMenu.WBP_MainMenu_C" _returnvalue))
  (UserInterface|Viewport|AddtoViewport _returnvalue_2 0)
  (Input|SetInputModeUIOnly _returnvalue _returnvalue_2 "DoNotLock" false)
  (Variables|/Script/Engine.PlayerController|SetbShowMouseCursor _returnvalue true))

(event Collision|EventActorBeginOverlap
  (params (OtherActor :type Actor%20Object%20Reference)))

(event EventTick
  (params (DeltaSeconds :type Float%20%28single-precision%29))
  (bind _niagarainitlocation (Variables|Default|GetNiagaraInitLocation))
  (CallFunction|UpdateTime DeltaSeconds)
  (Transformation|SetWorldLocation (Variables|Default|GetNiagara) (Math|Vector|MakeVector (.x _niagarainitlocation) (.y _niagarainitlocation) (+ (.z _niagarainitlocation) (CallFunction|SinValue))) false false)
  (Transformation|AddLocalRotation (Variables|Default|GetMagicDecal) (Math|Rotator|MakeRotator (* (Utilities|Time|GetWorldDeltaSeconds) 12.0) 0.0 0.0) false false))

(fn ConstructionScript)

(fn SinValue
  (return (* (Math|Trig|Sin(Radians) (Variables|Default|GetTime)) (Variables|Default|GetAlpha))))

(fn UpdateTime
  (params (A :type Float%20%28double-precision%29))
  (Variables|Default|SetTime (+ A (Variables|Default|GetTime)))
  (if (>= (Variables|Default|GetTime) 6.28)
    (Variables|Default|SetTime 0.0)))