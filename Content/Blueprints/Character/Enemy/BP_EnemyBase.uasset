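; BP_EnemyBase is an enemy character Blueprint that handles spawn, dissolve and target-facing presentation.
; On BeginPlay, a timeline uniformly scales the mesh.
; Two events each play their own timeline to drive the Dissolve scalar on a supplied dynamic material instance, with one dedicated to the weapon.
; UpdateFacingTarget feeds a location into Motion Warping as the FacingTarget warp target.
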(event EventBeginPlay
  (bind _scaletrack (Timeline|SpawnTimeline Play)
    (:Update
      (Transformation|SetRelativeScale3D (Variables|Character|GetMesh) (Math|Vector|MakeVector _scaletrack _scaletrack _scaletrack)))))

(event EventStartDissolveTimeLine
  (params (DynamicMaterialInstance :type Material%20Instance%20Dynamic%20Object%20Reference))
  (bind _dissolvetimeline (Timeline|DissolveTimeLine Play)
    (:Update
      (Rendering|Material|SetScalarParameterValue DynamicMaterialInstance "Dissolve" _dissolvetimeline :!class /Script/Engine.MaterialInstanceDynamic))))

(event EventStartWeaponDissolveTimeLine
  (params (DynamicMaterialInstance :type Material%20Instance%20Dynamic%20Object%20Reference))
  (bind _dissolveweapon (Timeline|DissolveWeapon Play)
    (:Update
      (Rendering|Material|SetScalarParameterValue DynamicMaterialInstance "Dissolve" _dissolveweapon :!class /Script/Engine.MaterialInstanceDynamic))))

(event EventUpdateFacingTarget
  (params (FacingTarget :type Vector%20%28by%20ref%29 :default "0, 0, 0"))
  (Class|MotionWarpingComponent|AddorUpdateWarpTargetfromLocation (Variables|Default|GetMotionWarping) "FacingTarget" FacingTarget))

(fn ConstructionScript)